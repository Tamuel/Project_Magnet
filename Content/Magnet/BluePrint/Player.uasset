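; Player Blueprint that steers a separate rolling Ball through device gravity input or the up/down and left/right axes.
; Each input applies torque to the ball scaled by RollTorque, with gravity readings offset by a stored calibration vector that SetCalibrateVector captures.
; It snaps its own location to the ball every tick and adds a test widget to the viewport on BeginPlay.
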(event `InputVectorAxis|Gravity`
  (params (AxisValue :type "Vector Structure"))
  (`PrimitiveComponent.AddTorque` (`/Game/Magnet/BluePrint/MagneticBall.Ball` (`self.Ball`)) (* (`KismetMathLibrary.MakeVector` (* -1 (.x (- AxisValue (`self.CalibrateVector`)))) (.y (- AxisValue (`self.CalibrateVector`)))) (`self.RollTorque`)) "None" false))

(event `InputAxis|UP_DOWN`
  (params (AxisValue :type "Float (single-precision)"))
  (`PrimitiveComponent.AddTorque` (`/Game/Magnet/BluePrint/MagneticBall.Ball` (`self.Ball`)) (`KismetMathLibrary.MakeVector` (* (`self.RollTorque`) AxisValue)) "None" false))

(event `InputAxis|LEFT_RIGHT`
  (params (AxisValue :type "Float (single-precision)"))
  (`PrimitiveComponent.AddTorque` (`/Game/Magnet/BluePrint/MagneticBall.Ball` (`self.Ball`)) (`KismetMathLibrary.MakeVector` 0.0 (* (`self.RollTorque`) AxisValue)) "None" false))

(event `self.ReceiveBeginPlay`
  (`self.Initialize`))

(event `self.ReceiveActorBeginOverlap`
  (params (OtherActor :type "Actor Object Reference")))

(event `self.ReceiveTick`
  (params (DeltaSeconds :type "Float (single-precision)"))
  (bind _ball (`self.Ball`))
  (`/Engine/EditorBlueprintResources/StandardMacros.IsValid` _ball
    (:`Is Valid`
      (`self.K2_SetActorLocation` (`SceneComponent.K2_GetComponentLocation` (`/Game/Magnet/BluePrint/MagneticBall.Ball` _ball))))))

(fn `GetGravityVector`
  (returns (returnVector :type "Vector Structure"))
  (return (`self.GetInputVectorAxisValue`)))

(fn `Initialize`
  (bind _returnvalue (`|CreateWidget` "/Game/Magnet/UI/TestWidget.TestWidget_C"))
  (`UserWidget.AddToViewport` _returnvalue 0))

(fn `SetCalibrateVector`
  (set `self.CalibrateVector` (`self.GetInputVectorAxisValue`)))

(fn `UserConstructionScript`)