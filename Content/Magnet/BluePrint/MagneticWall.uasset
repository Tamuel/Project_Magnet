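; MagneticWall is a wall actor whose look reflects its magnetism type.
; The construction script calls the parent's, then switches on Magnetism to set the Cube's material: basic wall for paramagnetic and ferromagnetic, dedicated pole materials for North and South.
; On BeginPlay it assigns the Cube and Sphere components to the Mesh and Collision references.
; The graph itself contains no magnetic force, overlap or tick logic.
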(event `self.ReceiveBeginPlay`
  (set `self.Mesh` (`self.Cube`))
  (set `self.Collision` (`self.Sphere`)))

(event `self.ReceiveActorBeginOverlap`
  (params (OtherActor :type "Actor Object Reference")))

(event `self.ReceiveTick`
  (params (DeltaSeconds :type "Float (single-precision)")))

(fn `UserConstructionScript`
  (bind _cube (`self.Cube`))
  (`parent.UserConstructionScript`)
  (switch `/Game/Magnet/BluePrint/MagnetismType` (`self.Magnetism`)
    (:`NewEnumerator0`
      (`PrimitiveComponent.SetMaterial` _cube 0 "/Game/MobileStarterContent/Materials/M_Basic_Wall.M_Basic_Wall" :!label _label))
    (:`NewEnumerator1`
      (goto _label))
    (:`NewEnumerator2`
      (`PrimitiveComponent.SetMaterial` _cube 0 "/Game/Magnet/Texture/NorthPolarTexture_Mat.NorthPolarTexture_Mat"))
    (:`NewEnumerator3`
      (`PrimitiveComponent.SetMaterial` _cube 0 "/Game/Magnet/Texture/SouthPolarTexture_Mat.SouthPolarTexture_Mat"))))