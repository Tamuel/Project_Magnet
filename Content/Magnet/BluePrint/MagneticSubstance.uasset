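; Magnetic actor that pulls or pushes other MagneticSubstance actors according to their Magnetism: North, South or Ferromagnetic.
; Overlap events track nearby substances, and Tick snaps the actor to its Mesh before applying forces.
; Like poles repel, opposite poles and pole-to-ferromagnetic pairs attract, and two ferromagnetics ignore each other.
; Each actor pushes both meshes along the unnormalized offset, scaled by MagneticForce and a linear distance falloff based on Collision radius.
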(event `self.ReceiveBeginPlay`)

(event `self.ReceiveActorBeginOverlap`
  (params (OtherActor :type "Actor Object Reference"))
  (bind _asmagnetic_substance (cast `/Game/Magnet/BluePrint/MagneticSubstance` OtherActor))
  (`KismetArrayLibrary.Array_Add` (`self.MagneticSubRefs`) _asmagnetic_substance))

(event `self.ReceiveActorEndOverlap`
  (params (OtherActor :type "Actor Object Reference"))
  (bind _asmagnetic_substance (cast `/Game/Magnet/BluePrint/MagneticSubstance` OtherActor))
  (`KismetArrayLibrary.Array_RemoveItem` (`self.MagneticSubRefs`) _asmagnetic_substance))

(event `self.ReceiveTick`
  (params (DeltaSeconds :type "Float (single-precision)"))
  (bind _returnvalue (`self.K2_GetActorLocation`))
  (bind _returnvalue_2 (`self.K2_GetActorLocation`))
  (bind _magneticsubrefs (`self.MagneticSubRefs`))
  (bind _magnetism (`self.Magnetism`))
  (bind _mesh (`self.Mesh`))
  (bind _currentmagneticforce (`self.CurrentMagneticForce`))
  (bind _currentmagneticforce_2 (`self.CurrentMagneticForce`))
  (bind _returnvalue_3 (`SphereComponent.GetScaledSphereRadius` (`self.Collision`)))
  (`/Engine/EditorBlueprintResources/StandardMacros.IsValid` _mesh
    (:`Is Valid`
      (`self.K2_SetActorLocation` (`SceneComponent.K2_GetComponentLocation` _mesh))
      ;[1 1 1] 주변에 물체가 있는지
      (if (not (== (`KismetArrayLibrary.Array_Length` _magneticsubrefs) 0))
        ;[1 1 1] 인력, 척력 구현
        (for _array_element _magneticsubrefs
          (switch `/Game/Magnet/BluePrint/MagnetismType` (`/Game/Magnet/BluePrint/MagneticSubstance.Magnetism` _array_element)
            (:`NewEnumerator0`)
            (:`NewEnumerator1`
              ;;[1 1 1] 강자성체, 자성이 통하지만 극성은 없음 ex) 철
              (switch `/Game/Magnet/BluePrint/MagnetismType` _magnetism
                (:`NewEnumerator0`)
                (:`NewEnumerator1`)
                (:`NewEnumerator2`
                  _)
                (:`NewEnumerator3`
                  _))
              (bind _returnvalue_4 (* (`self.MagneticForce`) (/ (- (* 5 _returnvalue_3) (`KismetMathLibrary.VSize` (- (`self.K2_GetActorLocation` _array_element) (`self.K2_GetActorLocation`)))) _returnvalue_3)))
              ;;[1 1 1] 인력, 당기는 힘
              (set `self.CurrentMagneticForce` _returnvalue_4 :!label _label)
              (bind _returnvalue_5 (`self.K2_GetActorLocation` _array_element))
              (`PrimitiveComponent.AddForce` (`self.Mesh`) (* (- _returnvalue_5 _returnvalue) _currentmagneticforce_2) "None" false)
              (`PrimitiveComponent.AddForce` (`/Game/Magnet/BluePrint/MagneticSubstance.Mesh` _array_element) (* (- _returnvalue _returnvalue_5) _currentmagneticforce_2) "None" false))
            (:`NewEnumerator2`
              ;;[1 1 1] 자성체, 극성을 가짐 ex) 자석
              (switch `/Game/Magnet/BluePrint/MagnetismType` _magnetism
                (:`NewEnumerator0`)
                (:`NewEnumerator1`
                  (goto _label))
                (:`NewEnumerator2`
                  ;;[1 1 1] 척력, 밀어내는 힘
                  (set `self.CurrentMagneticForce` _returnvalue_4 :!label _label_2)
                  (bind _returnvalue_6 (`self.K2_GetActorLocation` _array_element))
                  (`PrimitiveComponent.AddForce` (`self.Mesh`) (* (- _returnvalue_2 _returnvalue_6) _currentmagneticforce) "None" false)
                  (`PrimitiveComponent.AddForce` (`/Game/Magnet/BluePrint/MagneticSubstance.Mesh` _array_element) (* (- _returnvalue_6 _returnvalue_2) _currentmagneticforce) "None" false))
                (:`NewEnumerator3`
                  (goto _label))))
            (:`NewEnumerator3`
              (switch `/Game/Magnet/BluePrint/MagnetismType` _magnetism
                (:`NewEnumerator0`)
                (:`NewEnumerator1`
                  (goto _label))
                (:`NewEnumerator2`
                  (goto _label))
                (:`NewEnumerator3`
                  (goto _label_2))))))))))

(fn `UserConstructionScript`)