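; NoGravityArea is an overlap-driven zone that switches off gravity for actors inside it.
; Begin and end overlap disable and re-enable gravity on the overlapping actor's first StaticMeshComponent.
; When that actor is the referenced Player, the same events also set and clear its NoGravityCheck flag.
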(event `self.ReceiveBeginPlay`)

(event `self.ReceiveActorBeginOverlap`
  (params (OtherActor :type "Actor Object Reference"))
  (`PrimitiveComponent.SetEnableGravity` (`KismetArrayLibrary.Array_Get` (`self.K2_GetComponentsByClass` OtherActor "/Script/Engine.StaticMeshComponent")) false)
  (bind _asplayer (cast `/Game/Magnet/BluePrint/Player` OtherActor))
  (if (== _asplayer "/Game/Magnet/BluePrint/Player.Player")
    (set `/Game/Magnet/BluePrint/Player.NoGravityCheck` true _asplayer)))

(event `self.ReceiveActorEndOverlap`
  (params (OtherActor :type "Actor Object Reference"))
  (`PrimitiveComponent.SetEnableGravity` (`KismetArrayLibrary.Array_Get` (`self.K2_GetComponentsByClass` OtherActor "/Script/Engine.StaticMeshComponent")) true)
  (bind _asplayer (cast `/Game/Magnet/BluePrint/Player` OtherActor))
  (if (== _asplayer "/Game/Magnet/BluePrint/Player.Player")
    (set `/Game/Magnet/BluePrint/Player.NoGravityCheck` false _asplayer)))

(fn `UserConstructionScript`)